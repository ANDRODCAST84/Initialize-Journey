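; CameraManager switches the player's view between the world player camera and two battle cameras, normal and zoomed.
; On BeginPlay it retries every short delay until the first player controller's pawn casts to WorldPlayer, then caches it.
; Three focus events pass either that pawn or a named CameraList entry to ChangeCamera.
; ChangeCamera calls SetViewTargetWithBlend on the first player controller without specifying blend settings.
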(event `self.ReceiveBeginPlay`
  (bind _asworld_player (cast `/Game/Blueprints/WorldBlueprints/WorldPlayer` (`Controller.K2_GetPawn` (`GameplayStatics.GetPlayerController` 0)) :!label _label)
    (:`then`
      (set `self.WorldPlayer` _asworld_player))
    (:`CastFailed`
      (`KismetSystemLibrary.Delay` 0.2)
      (goto _label))))

(event `FocusWorldPlyaerCam`
  (`self.ChangeCamera` (`self.WorldPlayer`)))

(event `FocusBattleCam`
  (`self.ChangeCamera` (`BlueprintMapLibrary.Map_Find` (`self.CameraList`) "BattleCam")))

(event `FocusBattleZoomCam`
  (`self.ChangeCamera` (`BlueprintMapLibrary.Map_Find` (`self.CameraList`) "BattleZoomCam")))

(fn `ChangeCamera`
  (params (NewCam :type "Actor Object Reference"))
  (`PlayerController.SetViewTargetWithBlend` (`GameplayStatics.GetPlayerController` 0) NewCam 0.0 "VTBlend_Linear" 0.0 false))

(fn `UserConstructionScript`)