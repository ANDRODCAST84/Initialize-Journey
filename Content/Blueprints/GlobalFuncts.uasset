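; GlobalFuncts is a set of shared helper functions for switching the game between world, battle and dialogue states.
; Control helpers swap Enhanced Input mapping contexts on player 0, while camera helpers forward focus requests to the CameraManager actor.
; Getters return the core HUD and AudioManager.
; GO_TO_BATTLE uses that HUD to show the battle error popup widget, revealing an indexed image while a counter is below its limit.
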(fn `ChangeToBattleControls`
  (bind _returnvalue (pcsubsystem `EnhancedInputLocalPlayerSubsystem` (`GameplayStatics.GetPlayerController` null)))
  (`/Engine/EditorBlueprintResources/StandardMacros.IsValid` _returnvalue
    (:`Is Valid`
      (`EnhancedInputSubsystemInterface.RemoveMappingContext` _returnvalue "/Game/Blueprints/InputBlueprints/MovementInput/Movement.Movement" (struct))
      (`EnhancedInputSubsystemInterface.AddMappingContext` _returnvalue "/Game/Blueprints/InputBlueprints/BattleInput/Battle.Battle" 0 (struct)))))

(fn `ChangeToWorldControls`
  (bind _returnvalue (pcsubsystem `EnhancedInputLocalPlayerSubsystem` (`GameplayStatics.GetPlayerController` null)))
  (`/Engine/EditorBlueprintResources/StandardMacros.IsValid` _returnvalue
    (:`Is Valid`
      (`EnhancedInputSubsystemInterface.RemoveMappingContext` _returnvalue "/Game/Blueprints/InputBlueprints/BattleInput/Battle.Battle" (struct))
      (`EnhancedInputSubsystemInterface.AddMappingContext` _returnvalue "/Game/Blueprints/InputBlueprints/MovementInput/Movement.Movement" 0 (struct)))))

(fn `DialogueToWorldControls`
  (bind _returnvalue (pcsubsystem `EnhancedInputLocalPlayerSubsystem` (`GameplayStatics.GetPlayerController` null)))
  (`/Engine/EditorBlueprintResources/StandardMacros.IsValid` _returnvalue
    (:`Is Valid`
      (`EnhancedInputSubsystemInterface.RemoveMappingContext` _returnvalue "/Game/Blueprints/InputBlueprints/DialogueInput/DialogueMapping.DialogueMapping" (struct))
      (`EnhancedInputSubsystemInterface.AddMappingContext` _returnvalue "/Game/Blueprints/InputBlueprints/MovementInput/Movement.Movement" 0 (struct)))))

(fn `FocusBattleCam`
  (bind _returnvalue (`GameplayStatics.GetActorOfClass` null "/Game/Blueprints/CameraManager.CameraManager_C"))
  (`/Game/Blueprints/CameraManager.FocusBattleCam` _returnvalue))

(fn `FocusBattleZoomCam`
  (bind _returnvalue (`GameplayStatics.GetActorOfClass` null "/Game/Blueprints/CameraManager.CameraManager_C"))
  (`/Game/Blueprints/CameraManager.FocusBattleZoomCam` _returnvalue))

(fn `FocusWorldPlayerCam`
  (bind _returnvalue (`GameplayStatics.GetActorOfClass` null "/Game/Blueprints/CameraManager.CameraManager_C"))
  (`/Game/Blueprints/CameraManager.FocusWorldPlyaerCam` _returnvalue))

(fn `GetAudioManager`
  (returns (AudioManager :type "/Game/Blueprints/AudioManager Object Reference"))
  (bind _returnvalue (`GameplayStatics.GetActorOfClass` null "/Game/Blueprints/AudioManager.AudioManager_C"))
  (return _returnvalue))

(fn `GetBP_Core_HUD`
  (returns (return :type "/Game/Blueprints/BP_Core_HUD Object Reference"))
  (bind _asbp_core_hud (cast `/Game/Blueprints/BP_Core_HUD` (`PlayerController.GetHUD` (`GameplayStatics.GetPlayerController` null))))
  (return _asbp_core_hud))

(fn `GO_TO_BATTLE`
  (locals (Loopnum :type Integer))
  (bind _loopnum (`local.loopnum`))
  (bind _return (`self.GetBP_Core_HUD` null))
  (bind _battlepopups (`/Game/Blueprints/BP_Core_HUD.BattlePopups` _return))
  (bind _asbattle_error_popups (cast `/Game/Widgets/W_Blueprints/BattleErrorPopups` _battlepopups))
  (`Widget.SetVisibility` _battlepopups "HitTestInvisible")
  (if (< _loopnum 8)
    (`Widget.SetVisibility` (`|GetArrayItem` (`/Game/Widgets/W_Blueprints/BattleErrorPopups.ImgArray` _asbattle_error_popups) _loopnum) "HitTestInvisible")
    (`/Engine/EditorBlueprintResources/StandardMacros.IncrementInt` (`local.loopnum`))))

(fn `WorldToDialogueControls`
  (bind _returnvalue (pcsubsystem `EnhancedInputLocalPlayerSubsystem` (`GameplayStatics.GetPlayerController` null)))
  (`/Engine/EditorBlueprintResources/StandardMacros.IsValid` _returnvalue
    (:`Is Valid`
      (`EnhancedInputSubsystemInterface.RemoveMappingContext` _returnvalue "/Game/Blueprints/InputBlueprints/MovementInput/Movement.Movement" (struct))
      (`EnhancedInputSubsystemInterface.AddMappingContext` _returnvalue "/Game/Blueprints/InputBlueprints/DialogueInput/DialogueMapping.DialogueMapping" 0 (struct)))))