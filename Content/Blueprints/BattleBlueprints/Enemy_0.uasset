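; Battle-scene enemy slot that becomes the world enemy's configured combatant and turns its sprite with the battle player's angle.
; BattleStart spawns an enemy data object to set animations and stats, then adds the AI component from a data table.
; TakeDamage briefly shows health and damage, then FinishDamage resumes AI or, at zero health, returns to world play, with dialogue hooks for BrokenAI.
; On destruction, it spawns a fresh Enemy_0.
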(event `self.ReceiveBeginPlay`
  (`SceneComponent.SetVisibility` (`self.HealthBar`) false false))

(event `BattleStart`
  (params (`World Enemy` :type "/Game/Blueprints/WorldBlueprints/WorldEnemy Object Reference"))
  (bind _output_get (set `self.WorldEnemy` `World Enemy`))
  (bind _output (`|GetArrayItem` (`/Game/Blueprints/WorldBlueprints/WorldEnemy.EnemyID_IN` _output_get) (`self.EnemyNumber`)))
  (if (!= _output -1)
    (bind _returnvalue (`|SpawnActorFromClass` "/Game/Blueprints/BattleBlueprints/EnemyClass.EnemyClass_C" (`self.Spawn Transform`) "Undefined" "MultiplyWithRoot" null null))
    (bind _output_get_2 (set `self.Enemy` _returnvalue))
    (`/Game/Blueprints/BattleBlueprints/EnemyClass.ConfigureProperties` _output_get_2 _output)
    (`self.SetAnimations` _output_get_2)
    (`/Game/Blueprints/BattleBlueprints/EnemyClass.ConfigureStats` _output_get_2 _output)
    (bind (_enemystats_enemyid _enemystats_health) (break `/Game/Blueprints/BattleBlueprints/EnemyBaseStatsStruct` (`/Game/Blueprints/BattleBlueprints/EnemyClass.EnemyStats` _output_get_2)))
    (bind _output_get_3 (set `self.MaxHealth` (`KismetMathLibrary.Conv_IntToDouble` _enemystats_health)))
    (set `self.CurrentHealth` _output_get_3)
    (bind _returnvalue_2 (`|GetDataTableRow` "/Game/DataTables/EnemyProperties_-_Sheet1.EnemyProperties_-_Sheet1" (`KismetStringLibrary.Conv_StringToName` (`KismetStringLibrary.Conv_IntToString` _output)))
      (:`then`
        (`|AddComponentByClass` (`.enemyAI_25_7DC3548C48404E9AD3CFB19E684F3E7F` (break `/Game/Blueprints/BattleBlueprints/EnemyPropertiesStruct` _returnvalue_2)))
        (bind _returnvalue_3 (`GameplayStatics.GetActorOfClass` "/Game/Blueprints/BattleBlueprints/BattlePlayer.BattlePlayer_C"))
        (set `self.BattlePlayer` _returnvalue_3)
        (set `self.battleStarted` true)))))

(event `self.ReceiveTick`
  (params (DeltaSeconds :type "Float (single-precision)"))
  (if (`self.battleStarted`)
    (`SceneComponent.K2_SetRelativeRotation` (`self.Sprite`) (`KismetMathLibrary.MakeRotator` 0.0 0.0 (- (`/Game/Blueprints/BattleBlueprints/BattlePlayer.currentAngle` (`self.BattlePlayer`)) 180.0)) false false)))

(event `self.ReceiveDestroyed`
  (`|SpawnActorFromClass` "Enemy_0_C" (`self.Spawn Transform`) "Undefined" "MultiplyWithRoot" null null))

(fn `FinishDamage`
  (locals (Transform :type "Transform Structure"))
  (bind _returnvalue (`self.GetComponentByClass` "/Game/ENEMIY_AI/BrokenAI.BrokenAI_C"))
  (bind _returnvalue_2 (`KismetSystemLibrary.IsValid` _returnvalue))
  (if _returnvalue_2
    (if (== (`self.CurrentHealth`) 1.0)
      (`/Game/ENEMIY_AI/BrokenAI.ActivateAutoDialogue` _returnvalue)))
  (`SceneComponent.SetVisibility` (`self.HealthBar`) false false)
  (`TextRenderComponent.K2_SetText` (`self.DamageNumber`) (`KismetTextLibrary.GetEmptyText`))
  (if (== (`self.CurrentHealth`) 0.0)
    (set `local.Transform` (`self.GetTransform`))
    (if (`KismetSystemLibrary.IsValid` (`self.GetComponentByClass` "/Game/ENEMIY_AI/BrokenAI.BrokenAI_C"))
      (bind _return (`/Game/Blueprints/GlobalFuncts.GetBP_Core_HUD`))
      (`Widget.SetVisibility` (`/Game/Blueprints/BP_Core_HUD.WB_Dialogue` _return) "HitTestInvisible")
      (`/Game/Blueprints/GlobalFuncts.WorldToDialogueControls`))
    (`self.K2_DestroyActor` self)
    (`/Game/Blueprints/GlobalFuncts.ChangeToWorldControls`)
    (bind _return_2 (`/Game/Blueprints/GlobalFuncts.GetBP_Core_HUD`))
    (`/Game/Blueprints/BP_Core_HUD.Toggle_Core_HUD` _return_2)
    (bind _audiomanager (`/Game/Blueprints/GlobalFuncts.GetAudioManager`))
    (`/Game/Blueprints/AudioManager.PlayLevelMusic` _audiomanager)
    (bind _returnvalue_3 (`GameplayStatics.GetActorOfClass` "/Game/Blueprints/WorldBlueprints/WorldPlayer.WorldPlayer_C"))
    (`Controller.Possess` (`GameplayStatics.GetPlayerController` 0) _returnvalue_3)
    (elif (not _returnvalue_2)
      (set `self.AI_Active` true)
      (`/Game/Blueprints/EnemyAI.ResumeAI` (`self.GetComponentByClass` "/Game/Blueprints/EnemyAI.EnemyAI_C")))))

(fn `SetAnimations`
  (params (enemyClass :type "/Game/Blueprints/BattleBlueprints/EnemyClass Object Reference"))
  (`PaperZDAnimationComponent.SetAnimInstanceClass` (`self.AnimationComponent`) (`.enemyAnimations_22_F103A2C24544F909AA183BBB503F8752` (break `/Game/Blueprints/BattleBlueprints/EnemyPropertiesStruct` (`/Game/Blueprints/BattleBlueprints/EnemyClass.EnemyProperties` enemyClass)))))

(fn `TakeDamage`
  (params (DamageTaken :type "Float (double-precision)"))
  (locals (NewLocalVar :type "Float (double-precision)"))
  (bind _healthbar (`self.HealthBar`))
  (bind _returnvalue (- (`self.CurrentHealth`) DamageTaken))
  (if (<= _returnvalue 0.0)
    (set `self.CurrentHealth` 0.0)
    (bind _ashealth_bar (cast `/Game/Widgets/W_Blueprints/HealthBar` (`WidgetComponent.GetWidget` (`self.HealthBar`))))
    (`ProgressBar.SetPercent` (`/Game/Widgets/W_Blueprints/HealthBar.HealthBarSlider` _ashealth_bar) 0.0)
    (else
      (set `self.CurrentHealth` _returnvalue)
      (bind _ashealth_bar_2 (cast `/Game/Widgets/W_Blueprints/HealthBar` (`WidgetComponent.GetWidget` (`self.HealthBar`))))
      (`ProgressBar.SetPercent` (`/Game/Widgets/W_Blueprints/HealthBar.HealthBarSlider` _ashealth_bar_2) (/ (`self.CurrentHealth`) (`self.MaxHealth`)))))
  (`TextRenderComponent.K2_SetText` (`self.DamageNumber`) (`KismetTextLibrary.Conv_DoubleToText` DamageTaken "HalfToEven"))
  (`WidgetComponent.RequestRenderUpdate` _healthbar)
  (`SceneComponent.SetVisibility` _healthbar true false)
  (`KismetSystemLibrary.K2_SetTimer` null "FinishDamage" 1.5))

(fn `UserConstructionScript`)