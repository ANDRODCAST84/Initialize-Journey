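; BattlePlayerMC is the player pawn for battles, using a sprite and spring arm, with movement apparently still in progress.
; On BeginPlay it adds the Battle Enhanced Input mapping context, but the BattleMove event does nothing.
; Disconnected nodes sketch circular movement around BattleCenter, turning an input-driven angle into location, control rotation, and sprite and spring arm yaw.
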(event `self.ReceiveBeginPlay`
  (bind _asplayer_controller (cast `PlayerController` (`self.GetController`)))
  (bind _returnvalue (pcsubsystem `EnhancedInputLocalPlayerSubsystem` _asplayer_controller))
  (`/Engine/EditorBlueprintResources/StandardMacros.IsValid` _returnvalue
    (:`Is Valid`
      (`EnhancedInputSubsystemInterface.AddMappingContext` _returnvalue "/Game/Blueprints/InputBlueprints/BattleInput/Battle.Battle" 1 (struct)))))

(event `EnhancedInput|/Game/Blueprints/InputBlueprints/BattleInput/BattleMove`
  (params (ActionValue :type "Float (double-precision)") (ElapsedSeconds :type "Float (double-precision)") (TriggeredSeconds :type "Float (double-precision)") (InputAction :type "InputAction Object Reference" :default "/Game/Blueprints/InputBlueprints/BattleInput/BattleMove.BattleMove")))

(fn `UserConstructionScript`)