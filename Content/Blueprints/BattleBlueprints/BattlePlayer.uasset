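; Player actor for battles, handling basic attack and parry input against a HUD action meter.
; BeginPlay caches the meter, adds the Battle mapping context and gathers enemies.
; Attack only spends meter or flashes it when short; parry halts a parryable enemy's AI, fires an EventHandler parry event, and attempts a half-meter cost regardless.
; Meter regeneration, orbit movement and directional input are disconnected; TakeDamage is empty.
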(event `self.ReceiveBeginPlay`
  (bind _return (`/Game/Blueprints/GlobalFuncts.GetBP_Core_HUD`))
  (bind _asaction_meter (cast `/Game/Widgets/W_Blueprints/ActionMeter` (`/Game/Blueprints/BP_Core_HUD.Action Meter` _return)))
  (set `self.ActionMeter` _asaction_meter)
  (bind _asplayer_controller (cast `PlayerController` (`self.GetController`)))
  (bind _returnvalue (pcsubsystem `EnhancedInputLocalPlayerSubsystem` _asplayer_controller))
  (`/Engine/EditorBlueprintResources/StandardMacros.IsValid` _returnvalue
    (:`Is Valid`
      (`EnhancedInputSubsystemInterface.AddMappingContext` _returnvalue "/Game/Blueprints/InputBlueprints/BattleInput/Battle.Battle" 1 (struct))
      (bind _outactors (`GameplayStatics.GetAllActorsOfClass` "/Game/Blueprints/BattleBlueprints/Enemy_0.Enemy_0_C"))
      (set `self.Enemies` _outactors))))

(event `self.ReceiveTick`
  (params (DeltaSeconds :type "Float (single-precision)")))

(event `EnhancedInput|/Game/Blueprints/InputBlueprints/BattleInput/BattleMove`
  (params (ActionValue :type "Float (double-precision)") (ElapsedSeconds :type "Float (double-precision)") (TriggeredSeconds :type "Float (double-precision)") (InputAction :type "InputAction Object Reference" :default "/Game/Blueprints/InputBlueprints/BattleInput/BattleMove.BattleMove")))

(event `EnhancedInput|/Game/Blueprints/InputBlueprints/BattleInput/BattleBasicAttack`
  (params (ActionValue :type Boolean) (ElapsedSeconds :type "Float (double-precision)") (TriggeredSeconds :type "Float (double-precision)") (InputAction :type "InputAction Object Reference" :default "/Game/Blueprints/InputBlueprints/BattleInput/BattleBasicAttack.BattleBasicAttack"))
  (bind _returnvalue (- (`self.ActionMeterAmount`) 15.0))
  (bind _actionmeterbar (`/Game/Widgets/W_Blueprints/ActionMeter.ActionMeterBar` (`self.ActionMeter`)))
  (:`Started`
    (`KismetSystemLibrary.PrintString` "Attack!")
    (if (< _returnvalue 0.0)
      (`ProgressBar.SetFillColorAndOpacity` (`/Game/Widgets/W_Blueprints/ActionMeter.ActionMeterBar` (`self.ActionMeter`)) (struct :`R` 1.0 :`G` 0.141176 :`B` 0.160784 :`A` 1.0))
      (`KismetSystemLibrary.Delay` 0.15)
      (`ProgressBar.SetFillColorAndOpacity` _actionmeterbar (struct :`R` 0.062745 :`G` 1.0 :`B` 0.023529 :`A` 1.0))
      (`KismetSystemLibrary.Delay` 0.15)
      (`ProgressBar.SetFillColorAndOpacity` _actionmeterbar (struct :`R` 1.0 :`G` 0.141176 :`B` 0.160784 :`A` 1.0))
      (`KismetSystemLibrary.Delay` 0.15)
      (`ProgressBar.SetFillColorAndOpacity` _actionmeterbar (struct :`R` 0.062745 :`G` 1.0 :`B` 0.023529 :`A` 1.0))
      (else
        (set `self.ActionMeterAmount` _returnvalue)))))

(event `EnhancedInput|/Game/Blueprints/InputBlueprints/BattleInput/BattleParry`
  (params (ActionValue :type Boolean) (ElapsedSeconds :type "Float (double-precision)") (TriggeredSeconds :type "Float (double-precision)") (InputAction :type "InputAction Object Reference" :default "/Game/Blueprints/InputBlueprints/BattleInput/BattleParry.BattleParry"))
  (:`Started`
    (bind _returnvalue (`GameplayStatics.GetActorOfClass` "/Game/Blueprints/BattleBlueprints/Enemy_0.Enemy_0_C"))
    (if (`/Game/Blueprints/BattleBlueprints/Enemy_0.CanParry` _returnvalue)
      (set `/Game/Blueprints/BattleBlueprints/Enemy_0.AI_Active` false _returnvalue)
      (bind _returnvalue_2 (`GameplayStatics.GetActorOfClass` "/Game/Events/DialogueEvents/EventHandler.EventHandler_C"))
      (bind _returnvalue_3 (`|AddComponentByClass` _returnvalue_2 "/Game/Blueprints/ParryEvent.ParryEvent_C"))
      (`/Game/Blueprints/ParryEvent.Call Parry` _returnvalue_3 _returnvalue))
    (set `self.Parrying` false)
    (`self.Check and Consume Meter` (* (`self.ActionMeterMax`) 0.5))))

(event `EnhancedInput|/Game/Blueprints/InputBlueprints/BattleInput/BattleActionSelect`
  (params (ActionValue :type "Vector2D Structure") (ElapsedSeconds :type "Float (double-precision)") (TriggeredSeconds :type "Float (double-precision)") (InputAction :type "InputAction Object Reference" :default "/Game/Blueprints/InputBlueprints/BattleInput/BattleActionSelect.BattleActionSelect")))

(fn `Check and Consume Meter`
  (params (Amount :type "Float (double-precision)"))
  (bind _returnvalue (- (`self.ActionMeterAmount`) Amount))
  (bind _actionmeterbar (`/Game/Widgets/W_Blueprints/ActionMeter.ActionMeterBar` (`self.ActionMeter`)))
  (if (< _returnvalue 0.0)
    (`ProgressBar.SetFillColorAndOpacity` _actionmeterbar (struct :`R` 1.0 :`G` 0.141176 :`B` 0.160784 :`A` 1.0))
    (`ProgressBar.SetFillColorAndOpacity` _actionmeterbar (struct :`R` 0.062745 :`G` 1.0 :`B` 0.023529 :`A` 1.0))
    (`ProgressBar.SetFillColorAndOpacity` _actionmeterbar (struct :`R` 1.0 :`G` 0.141176 :`B` 0.160784 :`A` 1.0))
    (`ProgressBar.SetFillColorAndOpacity` _actionmeterbar (struct :`R` 0.062745 :`G` 1.0 :`B` 0.023529 :`A` 1.0))
    (else
      (bind _output_get (set `self.ActionMeterAmount` _returnvalue))
      (`ProgressBar.SetPercent` (`/Game/Widgets/W_Blueprints/ActionMeter.ActionMeterBar` (`self.ActionMeter`)) (/ _output_get (`self.ActionMeterMax`)))
      (set `TextBlock.Text` (`KismetTextLibrary.Conv_Int64ToText` (`KismetMathLibrary.FFloor64` (`self.ActionMeterAmount`))) (`/Game/Widgets/W_Blueprints/ActionMeter.ActionMeterText` (`self.ActionMeter`)))
      (if (< (`self.ActionMeterAmount`) (`self.ActionMeterMax`))
        (if (> (+ (`self.ActionMeterAmount`) 0.1) (`self.ActionMeterMax`))
          (set `self.ActionMeterAmount` (`self.ActionMeterMax`))
          (else
            (set `self.ActionMeterAmount` 0.0)))))))

(fn `Enemy Missed`
  (locals (PlayerLocation :type "Vector Structure" :default (0.0 0.0 0.0)))
  (set `local.PlayerLocation` (`self.K2_GetActorLocation`))
  (`SceneComponent.SetVisibility` (`self.Miss!`) true false)
  (`TimelineComponent.PlayFromStart` (`self.Timeline`)))

(fn `TakeDamage`
  (params (DamageTaken :type "Float (double-precision)")))

(fn `UserConstructionScript`)