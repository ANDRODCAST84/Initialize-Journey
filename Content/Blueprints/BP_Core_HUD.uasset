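; BP_Core_HUD is the HUD Blueprint that creates and toggles the core world UI, action meter, battle focus and battle error popup widgets.
; BeginPlay adds all four to the viewport, tracking all but the popups in two arrays.
; Toggle events call ToggleWidget, which collapses other widgets in that array and switches input between game-only and game-and-UI.
; FocusGame always collapses the battle focus widget, whichever widget was toggled.
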(event `self.ReceiveBeginPlay`
  (`|ExecutionSequence`
    (:`then_0`
      (bind _returnvalue (`|CreateWidget` "/Game/Widgets/W_Blueprints/BattleErrorPopups.BattleErrorPopups_C" (`self.GetOwningPlayerController`)))
      (bind _output_get (set `self.BattlePopups` _returnvalue))
      (`UserWidget.AddToViewport` _output_get 0))
    (:`then_1`
      (`WidgetBlueprintLibrary.SetInputMode_GameOnly` (`self.GetOwningPlayerController`))
      (bind _returnvalue_2 (`|CreateWidget` "/Game/Widgets/W_Blueprints/World_UI.World_UI_C" (`self.GetOwningPlayerController`)))
      (bind _output_get_2 (set `self.BP_Core_HUD` _returnvalue_2))
      (`KismetArrayLibrary.Array_Add` (`self.HUD_List`) _output_get_2)
      (bind _returnvalue_3 (`|CreateWidget` "/Game/Widgets/W_Blueprints/ActionMeter.ActionMeter_C" (`self.GetOwningPlayerController`)))
      (bind _output_get_3 (set `self.Action Meter` _returnvalue_3))
      (`KismetArrayLibrary.Array_Add` (`self.HUD_List`) _output_get_3)
      (for _array_element (`self.HUD_List`)
        (`UserWidget.AddToViewport` _array_element 0)))
    (:`then_2`
      (bind _returnvalue_4 (`|CreateWidget` "/Game/Widgets/W_Blueprints/MCBattleFocus.MCBattleFocus_C" (`self.GetOwningPlayerController`)))
      (bind _output_get_4 (set `self.WB_BattleFocusUI` _returnvalue_4))
      (`KismetArrayLibrary.Array_Add` (`self.GameUI_List`) _output_get_4)
      (for _array_element_2 (`self.GameUI_List`)
        (`UserWidget.AddToViewport` _array_element_2 0)))))

(event `Toggle_BattleUI`
  (`self.Toggle Widget` (`self.Action Meter`) (`self.HUD_List`)))

(event `Toggle_Core_HUD`
  (`self.Toggle Widget` (`self.BP_Core_HUD`) (`self.HUD_List`)))

(event `Toggle_BattleFocusUI`
  (`self.Toggle Widget` (`self.WB_BattleFocusUI`) (`self.GameUI_List`)))

(fn `FocusGame`
  (`Widget.SetVisibility` (`self.WB_BattleFocusUI`) "Collapsed")
  (`WidgetBlueprintLibrary.SetInputMode_GameOnly` (`self.GetOwningPlayerController`)))

(fn `FocusWidget`
  (`Widget.SetVisibility` (`self.Widget_to_focus`) "SelfHitTestInvisible")
  (`WidgetBlueprintLibrary.SetInputMode_GameAndUIEx` (`self.GetOwningPlayerController`) (`self.Widget_to_focus`)))

(fn `Toggle Widget`
  (params (`Widget to focus` :type "UserWidget Object Reference") (`Widget Array` :type "Array of UserWidget Object Reference"))
  (`/Engine/EditorBlueprintResources/StandardMacros.IsValid` `Widget to focus`
    (:`Is Valid`
      (set `self.Widget_to_focus` `Widget to focus`)
      (for _array_element `Widget Array`
        (`/Engine/EditorBlueprintResources/StandardMacros.IsValid` _array_element
          (:`Is Valid`
            (if (== (`self.Widget_to_focus`) _array_element)
              (if (`Widget.IsVisible` (`self.Widget_to_focus`))
                (`self.FocusGame`)
                (else
                  (`self.FocusWidget`)))
              (elif (`Widget.IsVisible` _array_element)
                (`Widget.SetVisibility` _array_element "Collapsed")))))))))

(fn `UserConstructionScript`)