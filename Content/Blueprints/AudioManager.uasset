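; AudioManager Blueprint that plays a battle start sound followed by battle music.
; BeginPlay adds two audio components, BattleStart and BattleMusic, and stops both immediately.
; BattleBegins plays BattleStart and raises the BattleStarting flag.
; Tick polls that flag, waits through a fixed Delay of about 1.6 seconds, then starts BattleMusic and clears the flag.
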(event `self.ReceiveBeginPlay`
  (bind _returnvalue (`AddComponent|NODE_AddAudioComponent-0`))
  (bind _output_get (set `self.BattleStart` _returnvalue))
  (`AudioComponent.Stop` _output_get)
  (bind _returnvalue_2 (`AddComponent|NODE_AddAudioComponent-1`))
  (bind _output_get_2 (set `self.BattleMusic` _returnvalue_2))
  (`AudioComponent.Stop` _output_get_2))

(event `self.ReceiveTick`
  (params (DeltaSeconds :type "Float (single-precision)"))
  (if (`self.BattleStarting`)
    (`KismetSystemLibrary.Delay` 1.58)
    (`AudioComponent.Play` (`self.BattleMusic`) 0.0)
    (set `self.BattleStarting` false)))

(fn `BattleBegins`
  (`AudioComponent.Play` (`self.BattleStart`) 0.0)
  (set `self.BattleStarting` true))

(fn `UserConstructionScript`)