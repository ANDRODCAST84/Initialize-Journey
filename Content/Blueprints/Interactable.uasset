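; Interactable is an actor that shows a popup when the player can interact with it and delegates the interaction to a script component.
; On BeginPlay it adds a component of the InteractScript class and stores it as ConcreteInteractScript.
; Overlap events toggle InteractPopup visibility for actors tagged Player.
; CallInteractScript forwards to the component's CallScript, so behavior lives in the component rather than the actor.
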(event `self.ReceiveBeginPlay`
  (bind _returnvalue (`|AddComponentByClass` (`self.InteractScript`)))
  (set `self.ConcreteInteractScript` _returnvalue))

(event `self.ReceiveActorEndOverlap`
  (params (OtherActor :type "Actor Object Reference"))
  (if (`self.ActorHasTag` OtherActor "Player")
    (`SceneComponent.SetVisibility` (`self.InteractPopup`) false false)))

(event `self.ReceiveActorBeginOverlap`
  (params (OtherActor :type "Actor Object Reference"))
  (if (`self.ActorHasTag` OtherActor "Player")
    (`SceneComponent.SetVisibility` (`self.InteractPopup`) true false)))

(fn `Call_InteractScript`
  (`/Game/Blueprints/interactScript.CallScript` (`self.ConcreteInteractScript`)))

(fn `UserConstructionScript`)