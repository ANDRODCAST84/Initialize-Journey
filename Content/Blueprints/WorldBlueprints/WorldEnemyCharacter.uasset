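; WorldEnemyCharacter is an overworld enemy that starts a battle the first time an actor overlaps it.
; On BeginPlay it spawns a WorldEnemy from its enemy ID, and on overlap passes that actor the Enemy_0 found in the level.
; The transition switches controls and audio, reveals HUD error popups one by one on a looping timer, then hides them.
; It then triggers the WorldEnemy's battle event, toggles battle UI and possesses the BattlePlayer.
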(event `self.ReceiveBeginPlay`
  (bind _returnvalue (`|SpawnActorFromClass` "/Game/Blueprints/WorldBlueprints/WorldEnemy.WorldEnemy_C" (`self.Spawn Transform`) "Undefined" "MultiplyWithRoot" null (`self.EnemyID_IN`) null))
  (set `self.WorldEnemy` _returnvalue))

(event `self.ReceiveActorBeginOverlap`
  (params (OtherActor :type "Actor Object Reference"))
  (bind _returnvalue (`GameplayStatics.GetActorOfClass` "/Game/Blueprints/BattleBlueprints/Enemy_0.Enemy_0_C"))
  (bind _output_get (set `self.Enemy_0` _returnvalue))
  (set `/Game/Blueprints/WorldBlueprints/WorldEnemy.Enemy_0` _output_get (`self.WorldEnemy`))
  (if (not (`self.OVERLAPPED`))
    (set `self.OVERLAPPED` true)
    (set `self.BattleTriggered` true)
    (`/Game/Blueprints/GlobalFuncts.ChangeToBattleControls`)
    (`KismetSystemLibrary.K2_SetTimer` null "POPUPS" 0.18 true)
    (bind _return (`/Game/Blueprints/GlobalFuncts.GetBP_Core_HUD`))
    (bind _audiomanager (`/Game/Blueprints/GlobalFuncts.GetAudioManager`))
    (`/Game/Blueprints/AudioManager.BattleBegins` _audiomanager)
    (`self.POPUPS`)
    (`KismetSystemLibrary.Delay` 1.6)
    (`KismetSystemLibrary.K2_SetTimer` null "POPUPS" 0.0 true)
    (`/Game/Blueprints/GlobalFuncts.GetBP_Core_HUD`)
    (bind _asbattle_error_popups (cast `/Game/Widgets/W_Blueprints/BattleErrorPopups` (`/Game/Blueprints/BP_Core_HUD.BattlePopups` _return)))
    (for _array_element (`/Game/Widgets/W_Blueprints/BattleErrorPopups.ImgArray` _asbattle_error_popups)
      (`Widget.SetVisibility` _array_element "Collapsed")
      (`Widget.SetVisibility` (`/Game/Blueprints/BP_Core_HUD.BattlePopups` _return) "Collapsed"))
    (`/Game/Blueprints/WorldBlueprints/WorldEnemy.BattleTriggeredEvent` (`self.WorldEnemy`))
    (`/Game/Blueprints/BP_Core_HUD.Toggle_BattleUI` _return)
    (bind _returnvalue_2 (`GameplayStatics.GetActorOfClass` "/Game/Blueprints/BattleBlueprints/BattlePlayer.BattlePlayer_C"))
    (`Controller.Possess` (`GameplayStatics.GetPlayerController` 0) _returnvalue_2)
    (set `/Game/Blueprints/BattleBlueprints/BattlePlayer.inBattle` true _returnvalue_2)))

(fn `POPUPS`
  (bind _loopnum (`self.loopnum`))
  (bind _return (`/Game/Blueprints/GlobalFuncts.GetBP_Core_HUD`))
  (bind _battlepopups (`/Game/Blueprints/BP_Core_HUD.BattlePopups` _return))
  (bind _asbattle_error_popups (cast `/Game/Widgets/W_Blueprints/BattleErrorPopups` _battlepopups))
  (`Widget.SetVisibility` _battlepopups "HitTestInvisible")
  (if (< _loopnum 8)
    (`Widget.SetVisibility` (`|GetArrayItem` (`/Game/Widgets/W_Blueprints/BattleErrorPopups.ImgArray` _asbattle_error_popups) _loopnum) "HitTestInvisible")
    (`/Engine/EditorBlueprintResources/StandardMacros.IncrementInt` (`self.loopnum`))))

(fn `UserConstructionScript`)