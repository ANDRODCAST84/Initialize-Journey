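; Player character for a sprite-based world that handles movement, jumping and battle menu input.
; BeginPlay adds the Movement input context and caches the battle and battle-focus widgets from the core HUD.
; Confirm and escape inputs drive those widgets and track menu depth, with escape also refocusing the battle camera.
; Helper functions adjust the spring-arm camera from player position and step focus through a two-by-two option grid and character list.
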(event `self.ReceiveBeginPlay`
  (bind _asplayer_controller (cast `PlayerController` (`self.GetController`)))
  (bind _returnvalue (pcsubsystem `EnhancedInputLocalPlayerSubsystem` _asplayer_controller))
  (`/Engine/EditorBlueprintResources/StandardMacros.IsValid` _returnvalue
    (:`Is Valid`
      (`EnhancedInputSubsystemInterface.AddMappingContext` _returnvalue "/Game/Blueprints/InputBlueprints/MovementInput/Movement.Movement" 0 (struct))
      (bind _return (`/Game/Blueprints/GlobalFuncts.GetBP_Core_HUD`))
      (bind _output_get (set `self.BP_Core_HUD` _return))
      (bind _asbattle_ui (cast `/Game/Widgets/W_Blueprints/Battle_UI` (`/Game/Blueprints/BP_Core_HUD.WB_BattleUI` _output_get)))
      (bind _output_get_2 (set `self.BattleUI` _asbattle_ui))
      (`KismetArrayLibrary.Array_Add` (`self.BattleWidgets`) _output_get_2)
      (bind _asmcbattle_focus (cast `/Game/Widgets/W_Blueprints/MCBattleFocus` (`/Game/Blueprints/BP_Core_HUD.WB_BattleFocusUI` (`self.BP_Core_HUD`))))
      (bind _output_get_3 (set `self.BattleFocusUI` _asmcbattle_focus))
      (`KismetArrayLibrary.Array_Add` (`self.BattleWidgets`) _output_get_3))))

(event `EnhancedInput|/Game/Blueprints/InputBlueprints/MovementInput/HorizontaMove`
  (params (ActionValue :type "Float (double-precision)") (ElapsedSeconds :type "Float (double-precision)") (TriggeredSeconds :type "Float (double-precision)") (InputAction :type "InputAction Object Reference" :default "/Game/Blueprints/InputBlueprints/MovementInput/HorizontaMove.HorizontaMove"))
  (bind _sprite (`self.Sprite`))
  (:`Triggered`
    (`self.AddMovementInput` (0.0 0.3 0.0) ActionValue)
    (if (< ActionValue 0.0)
      (`SceneComponent.K2_SetRelativeRotation` :`self` _sprite)
      (else
        (`SceneComponent.K2_SetRelativeRotation` _sprite (struct :`Yaw` 180.0) false false)))))

(event `EnhancedInput|/Game/Blueprints/InputBlueprints/MovementInput/VerticalMove`
  (params (ActionValue :type "Float (double-precision)") (ElapsedSeconds :type "Float (double-precision)") (TriggeredSeconds :type "Float (double-precision)") (InputAction :type "InputAction Object Reference" :default "/Game/Blueprints/InputBlueprints/MovementInput/VerticalMove.VerticalMove"))
  (:`Triggered`
    (`self.AddMovementInput` (0.3 0.0 0.0) ActionValue)))

(event `EnhancedInput|/Game/Blueprints/InputBlueprints/MovementInput/JumpAction`
  (params (ActionValue :type Boolean) (ElapsedSeconds :type "Float (double-precision)") (TriggeredSeconds :type "Float (double-precision)") (InputAction :type "InputAction Object Reference" :default "/Game/Blueprints/InputBlueprints/MovementInput/JumpAction.JumpAction"))
  (:`Triggered`
    (`self.Jump`)
    (set `self.jumping` ActionValue)))

(event `self.ReceiveTick`
  (params (DeltaSeconds :type "Float (single-precision)")))

(event `EnhancedInput|/Game/Blueprints/InputBlueprints/BattleInput/MenuEscape`
  (params (ActionValue :type Boolean) (ElapsedSeconds :type "Float (double-precision)") (TriggeredSeconds :type "Float (double-precision)") (InputAction :type "InputAction Object Reference" :default "/Game/Blueprints/InputBlueprints/BattleInput/MenuEscape.MenuEscape"))
  (bind _battleui (`self.BattleUI`))
  (:`Started`
    (if ActionValue
      (`/Engine/EditorBlueprintResources/StandardMacros.DecrementInt` (`self.BattleW_Index`)
        (:`  `
          (switch `int` 0
            (:`0`
              (`/Game/Blueprints/BP_Core_HUD.Toggle_BattleUI` (`self.BP_Core_HUD`))
              (`/Game/Widgets/W_Blueprints/Battle_UI.UpdateFocusCharSelect` _battleui 0)
              (`/Game/Blueprints/GlobalFuncts.FocusBattleCam`)
              (`/Game/Widgets/W_Blueprints/Battle_UI.BattleTopDown` _battleui))))))))

(event `EnhancedInput|/Game/Blueprints/InputBlueprints/BattleInput/MenuConfirmation`
  (params (ActionValue :type Boolean) (ElapsedSeconds :type "Float (double-precision)") (TriggeredSeconds :type "Float (double-precision)") (InputAction :type "InputAction Object Reference" :default "/Game/Blueprints/InputBlueprints/BattleInput/MenuConfirmation.MenuConfirmation"))
  (bind _battleui (`self.BattleUI`))
  (bind _widget_to_focus (`/Game/Blueprints/BP_Core_HUD.Widget_to_focus` (`self.BP_Core_HUD`)))
  (:`Started`
    (if ActionValue
      (`/Engine/EditorBlueprintResources/StandardMacros.IncrementInt` (`self.BattleW_Index`)
        (:`  `
          (for (_array_element _array_index) (`self.BattleWidgets`)
            (if (== _array_element _widget_to_focus)
              (switch `int` _array_index
                (:`0`
                  (switch `int` (`/Game/Widgets/W_Blueprints/Battle_UI.CharButtonIndex` _battleui)
                    (:`0`
                      (`/Game/Widgets/W_Blueprints/Battle_UI.MainChar_Pressed` _battleui))))
                (:`1`
                  (cast `/Game/Widgets/W_Blueprints/MCBattleFocus` _widget_to_focus))))))))))

(fn `Adujst Camera`
  (bind _returnvalue (`self.GetTransform`))
  (bind _leftmargin (`self.LeftMargin`))
  (`|ExecutionSequence`
    (:`then_0`
      (set `SpringArmComponent.TargetArmLength` (- -520.0 (.x (.location _returnvalue))) (`self.SpringArm`)))
    (:`then_1`
      (if (>= (.y (.location _returnvalue)) _leftmargin)
        (set `SpringArmComponent.SocketOffset` (`KismetMathLibrary.MakeVector` 0.0 (- (.y (.location _returnvalue)) _leftmargin)) (`self.SpringArm`))))
    (:`then_2`
      (`SceneComponent.K2_SetRelativeTransform` (`SceneComponent.GetChildComponent` (`self.SpringArm`) 0) (`KismetMathLibrary.MakeTransform` (`KismetMathLibrary.MakeVector` 0.0 0.0 (- 260.0 (.z (.location _returnvalue))))) false false))))

(fn `UpdateCharSelect`
  (params (Y :type "Float (double-precision)"))
  (bind _charbuttonindex (`/Game/Widgets/W_Blueprints/Battle_UI.CharButtonIndex` (`self.BattleUI`)))
  (bind _charbuttonindex_2 (`/Game/Widgets/W_Blueprints/Battle_UI.CharButtonIndex` (`self.BattleUI`)))
  (if (== Y 1.0)
    (if (< _charbuttonindex_2 2)
      (`/Game/Widgets/W_Blueprints/Battle_UI.UpdateFocusCharSelect` (`self.BattleUI`) (+ _charbuttonindex_2 1)))
    (elif (== Y -1.0)
      (if (> _charbuttonindex 0)
        (`/Game/Widgets/W_Blueprints/Battle_UI.UpdateFocusCharSelect` (`self.BattleUI`) (- _charbuttonindex 1))))))

(fn `UpdateMainBattleOptions`
  (params (X :type "Float (double-precision)") (Y :type "Float (double-precision)"))
  (bind _mainbutten_i (`/Game/Widgets/W_Blueprints/MCBattleFocus.MainButten_i` (`self.BattleFocusUI`)))
  (bind _mainbutten_i_2 (`/Game/Widgets/W_Blueprints/MCBattleFocus.MainButten_i` (`self.BattleFocusUI`)))
  (bind _mainbutten_i_3 (`/Game/Widgets/W_Blueprints/MCBattleFocus.MainButten_i` (`self.BattleFocusUI`)))
  (bind _mainbutten_i_4 (`/Game/Widgets/W_Blueprints/MCBattleFocus.MainButten_i` (`self.BattleFocusUI`)))
  (`|ExecutionSequence`
    (:`then_0`
      (if (== X 1.0)
        (if (< _mainbutten_i 2)
          (`/Game/Widgets/W_Blueprints/MCBattleFocus.UpdateFocusMain` (`self.BattleFocusUI`) (+ _mainbutten_i 2)))
        (elif (== X -1.0)
          (if (> _mainbutten_i_2 1)
            (`/Game/Widgets/W_Blueprints/MCBattleFocus.UpdateFocusMain` (`self.BattleFocusUI`) (- _mainbutten_i_2 2))))))
    (:`then_1`
      (if (== Y 1.0)
        (if (or (== _mainbutten_i_3 0) (== _mainbutten_i_3 2))
          (`/Game/Widgets/W_Blueprints/MCBattleFocus.UpdateFocusMain` (`self.BattleFocusUI`) (+ _mainbutten_i_3 1)))
        (elif (== Y -1.0)
          (if (or (== _mainbutten_i_4 3) (== _mainbutten_i_4 1))
            (`/Game/Widgets/W_Blueprints/MCBattleFocus.UpdateFocusMain` (`self.BattleFocusUI`) (- _mainbutten_i_4 1))))))))

(fn `UserConstructionScript`)